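; BP_Gun is a gun actor that attaches itself to the player pawn, with firing logic that is not hooked up.
; On BeginPlay it enables input for player 0, snaps to the pawn's location and rotation, and applies a fixed relative offset.
; A disconnected chain would spawn a BP_Sphere at the gun's transform and print a debug message, but no event calls it.
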(event `self.ReceiveBeginPlay`
  (`self.EnableInput` (`GameplayStatics.GetPlayerController` 0))
  (`KismetSystemLibrary.PrintString` "GUN_READY")
  (`self.K2_AttachToActor` (`GameplayStatics.GetPlayerPawn` 0) "None" "SnapToTarget" "SnapToTarget" "KeepWorld")
  (`self.K2_SetActorRelativeLocation` (60.0 35.0 -15.0)))

(event `Key|LeftMouseButton`
  (params (Key :type "Key Structure")))

(fn `UserConstructionScript`)